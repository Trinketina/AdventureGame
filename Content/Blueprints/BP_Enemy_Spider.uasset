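; BP_Enemy_Spider is a spider enemy that roams at random and can be killed by damage.
; RandomRoam loops AI move-to calls toward random reachable points around its current location, pausing briefly after each success or failure.
; AnyDamage lowers health, briefly flashing a damage material on surviving hits.
; On death it decrements the BP_Adventure game mode's spider count, updates the UI enemy count and destroys itself.
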(event Custom|RandomRoam
  ;[1 1 1] movement
  (AI|AIMoveTo self (.RandomLocation (AI|Navigation|GetRandomReachablePointinRadius (Transformation|GetActorLocation) 4e+03 0 0)) 0 5.0 false
    (:OnSuccess
      _)
    (:OnFail
      _))
  (Utilities|FlowControl|Delay 2.0)
  (CallFunction|RandomRoam))

(event EventBeginPlay
  (Utilities|FlowControl|Sequence
    (:then_0
      (bind _asbp_adventure (Utilities|Casting|CastToBP_Adventure (Game|GetGameMode)))
      (Variables|Default|SetGamemode _asbp_adventure))
    (:then_1
      ;[1 1 1] movement
      (CallFunction|RandomRoam))))

(event Game|Damage|EventAnyDamage
  (params (Damage :type Float%20%28single-precision%29) (DamageType :type Damage%20Type%20Object%20Reference) (InstigatedBy :type Controller%20Object%20Reference) (DamageCauser :type Actor%20Object%20Reference))
  (bind _spider (Variables|Default|GetSpider))
  (bind _output_get (Variables|Default|SetSpiderHealth (- (Variables|Default|GetSpiderHealth) Damage)))
  (if (<= _output_get 0.0)
    (bind _result (Math|Integer|DecrementInt (Variables|/Game/Blueprints/BP_Adventure.BP_Adventure_C|GetspiderCount (Variables|Default|GetGamemode)))
      (:%20%20
        (Default|UpdateEnemyCount (Variables|/Game/Blueprints/BP_Adventure.BP_Adventure_C|GetUI (Variables|Default|GetGamemode)) _result)
        (Actor|DestroyActor)))
    (else
      (Rendering|Material|SetMaterial _spider 0 "/Game/EnemyAssets/MAT_Damage_Enemy.MAT_Damage_Enemy")
      (Utilities|FlowControl|Delay 0.2)
      (Rendering|Material|SetMaterial _spider 0 "/Game/EnemyAssets/03_-_Default.03_-_Default"))))

(fn ConstructionScript)